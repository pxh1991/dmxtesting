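; BP_LOC_ROT is a DMX fixture Blueprint that drives its own location and rotation from received DMX data.
; When the DMX component receives a fixture patch, it reads the attribute values and looks up one per axis.
; Each value is used as a Lerp alpha over a symmetric position or full-turn angle range, then applied directly to DefaultSceneRoot's relative transform, with no smoothing.
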(event OnFixturePatchReceived(DMX)
  (params (FixturePatch :type DMX%20Entity%20Fixture%20Patch%20Object%20Reference) (ValuePerAttribute :type DMX%20Normalized%20Attribute%20Value%20Map%20Structure%20%28by%20ref%29))
  (Class|DMXEntityFixturePatch|GetAttributesValues FixturePatch)
  (Transformation|SetRelativeLocationAndRotation (Variables|Default|GetDefaultSceneRoot) (Math|Vector|MakeVector (Math|Float|Lerp -8e+02 8e+02 (.Value (Utilities|Map|Find (.map ValuePerAttribute) "(Name=\"Location_X\")"))) (Math|Float|Lerp -8e+02 8e+02 (.Value (Utilities|Map|Find (.map ValuePerAttribute) "(Name=\"Location_Y\")"))) (Math|Float|Lerp -8e+02 8e+02 (.Value (Utilities|Map|Find (.map ValuePerAttribute) "(Name=\"Location_Z\")")))) (Math|Rotator|MakeRotator (Math|Float|Lerp -1.8e+02 1.8e+02 (.Value (Utilities|Map|Find (.map ValuePerAttribute) "(Name=\"Rotation_X\")"))) (Math|Float|Lerp -1.8e+02 1.8e+02 (.Value (Utilities|Map|Find (.map ValuePerAttribute) "(Name=\"Rotation_Y\")"))) (Math|Float|Lerp -1.8e+02 1.8e+02 (.Value (Utilities|Map|Find (.map ValuePerAttribute) "(Name=\"Rotation_Z\")")))) false false))

(event EventBeginPlay)

(event Collision|EventActorBeginOverlap
  (params (OtherActor :type Actor%20Object%20Reference)))

(event EventTick
  (params (DeltaSeconds :type Float%20%28single-precision%29)))

(fn ConstructionScript)