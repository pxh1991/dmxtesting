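; BP_FloorLine4 is a DMX floor line light fixture whose strip material follows the fixture's light color and dimmer.
; The construction script creates a dynamic instance of the Light1 material on StageSource31 after running the parent script.
; Every Tick, after the parent update, it copies the SpotLight color and the DimmerComponent's DMX target value into the material's strip color and dim parameters.
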(event EventBeginPlay
  (|CallParentFunction) ; 此节点被禁用，将不会被调用。\n从引脚连出引线来编译功能。
)

(event EventTick
  (params (DeltaSeconds :type Float%20%28single-precision%29))
  (bind _light_1_inst (Variables|Default|Getlight_1_inst))
  (|CallParentFunction DeltaSeconds)
  (Rendering|Material|SetVectorParameterValue _light_1_inst "strips_color" (Rendering|Components|Light|GetLightColor (Variables|Default|GetSpotLight)) :!class /Script/Engine.MaterialInstanceDynamic)
  (Rendering|Material|SetScalarParameterValue _light_1_inst "strips_dim" (* (Class|DMXFixtureComponentSingle|GetDMXTargetValue (Variables|Default|GetDimmer_Component)) 1.0) :!class /Script/Engine.MaterialInstanceDynamic))

(fn ConstructionScript
  (|CallParentFunction)
  (bind _returnvalue (Rendering|Material|CreateDynamicMaterialInstance (Variables|Default|Getstage_Source_31) 0 "/Game/FIX/light1.light1" "None" :!class /Script/Engine.PrimitiveComponent))
  (Variables|Default|Setlight_1_inst _returnvalue))