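; BP_SpotlightDMX is a spotlight fixture whose colour and beam width are driven by DMX data.
; When a fixture patch is received, it reads the attribute values and looks up individual channels in the resulting map.
; Each RGB component is an attribute value multiplied by a range-remapped attribute value, which sets the light colour.
; Another remapped value sets the outer cone angle, with the inner cone kept proportionally narrower.
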(event OnFixturePatchReceived(DMX)
  (params (FixturePatch :type DMX%20Entity%20Fixture%20Patch%20Object%20Reference) (ValuePerAttribute :type DMX%20Normalized%20Attribute%20Value%20Map%20Structure%20%28by%20ref%29))
  (bind _value (Utilities|Map|Find (.map ValuePerAttribute) "(Name=\"Dimmer\")"))
  (bind _value_2 (Utilities|Map|Find (.map ValuePerAttribute) "(Name=\"Zoom\")"))
  (bind _spotlightcomponent (Variables|Default|GetSpotLightComponent))
  (bind _returnvalue (Math|Float|MapRangeClamped _value_2 0.0 1.0 8.0 3e+01))
  (bind _returnvalue_2 (Math|Float|MapRangeClamped _value 0.0 255.0 0.0 1e+02))
  (Class|DMXEntityFixturePatch|GetAttributesValues FixturePatch)
  (Rendering|Components|Light|SetLightColor _spotlightcomponent (Utilities|Struct|MakeLinearColor (* (.Value (Utilities|Map|Find (.map ValuePerAttribute) "(Name=\"Red\")")) _returnvalue_2) (* (.Value (Utilities|Map|Find (.map ValuePerAttribute) "(Name=\"Green\")")) _returnvalue_2) (* (.Value (Utilities|Map|Find (.map ValuePerAttribute) "(Name=\"Blue\")")) _returnvalue_2) 1.0) true)
  (Rendering|Lighting|SetOuterConeAngle _spotlightcomponent _returnvalue)
  (Rendering|Lighting|SetInnerConeAngle _spotlightcomponent (* _returnvalue 0.8)))

(event EventBeginPlay)

(event EventTick
  (params (DeltaSeconds :type Float%20%28single-precision%29)))

(fn ConstructionScript)